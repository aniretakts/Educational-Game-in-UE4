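; Interactive board for the second room that runs a timed drag-form quiz and gates the door to the third room.
; Inside its trigger, the first Enter press opens the DragForm and Timer widgets in UI-only mode, then a fixed delay restores inventory and game input.
; Later presses reveal a text panel instead.
; Leaving the trigger sets the door flag and, guarded by Doonce, compares answers by index to compute and print a percentage score.
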(event `self.2ndRoomBoardTrigger.OnComponentBeginOverlap`
  (params (OverlappedComponent :type "PrimitiveComponent Object Reference") (OtherActor :type "Actor Object Reference") (OtherComp :type "PrimitiveComponent Object Reference") (OtherBodyIndex :type Integer) (bFromSweep :type Boolean) (SweepResult :type "HitResult Structure (by ref)"))
  (`self.EnableInput` (`GameplayStatics.GetPlayerController` 0))
  (set `self.DoorTo3rdRoom` false))

(event `self.2ndRoomBoardTrigger.OnComponentEndOverlap`
  (params (OverlappedComponent :type "PrimitiveComponent Object Reference") (OtherActor :type "Actor Object Reference") (OtherComp :type "PrimitiveComponent Object Reference") (OtherBodyIndex :type Integer))
  (`self.DisableInput` (`GameplayStatics.GetPlayerController` 0))
  (`SceneComponent.SetHiddenInGame` (`self.TextRender1`) true false)
  (`SceneComponent.SetHiddenInGame` (`self.Plane`) true false)
  (set `self.DoorTo3rdRoom` true)
  (if (`self.doonce`)
    (set `self.doonce` false)
    (for (_array_element _array_index) (`self.R2UsersAnswers`)
      (for (_array_element_2 _array_index_2) (`self.R2CorrectAnswers`)
        (if (== _array_index_2 _array_index)
          (if (`KismetStringLibrary.EqualEqual_StrStr` _array_element_2 _array_element)
            (set `self.R2NumofCorrectAnswers` (+ (`self.R2NumofCorrectAnswers`) 1))))))
    (set `self.R2Score` (`KismetMathLibrary.Conv_IntToDouble` (/ (* (`self.R2NumofCorrectAnswers`) 100) 7)))
    (`KismetSystemLibrary.PrintString` (`KismetStringLibrary.Conv_IntToString` (`self.R2NumofCorrectAnswers`)) true true (struct :`G` 0.66 :`B` 1.0 :`A` 1.0) 20.0)
    (`KismetSystemLibrary.PrintString` (`KismetStringLibrary.Conv_DoubleToString` (`self.R2Score`)) true true (struct :`R` 1.0 :`B` 0.938075 :`A` 1.0) 20.0)))

(event `Key|Enter`
  (params (Key :type "Key Structure"))
  (bind _returnvalue (`GameplayStatics.GetPlayerController` 0))
  (bind _returnvalue_2 (`GameplayStatics.GetPlayerController` 0))
  (:`Pressed`
    (`/Engine/EditorBlueprintResources/StandardMacros.IncrementInt` (`self.counter`)
      (:`  `
        (if (>= (`self.counter`) 2)
          (`SceneComponent.SetHiddenInGame` (`self.TextRender1`) false false)
          (`SceneComponent.SetHiddenInGame` (`self.Plane`) false false)
          (else
            (set `self.2ndRoomGameTriggered` true)
            (`WidgetLayoutLibrary.RemoveAllWidgets`)
            (bind _returnvalue_3 (`|CreateWidget` "/Game/Blueprints/Room_2/DragForm.DragForm_C"))
            (`UserWidget.AddToViewport` _returnvalue_3 0)
            (`WidgetBlueprintLibrary.SetInputMode_UIOnlyEx` _returnvalue null)
            (set `PlayerController.bShowMouseCursor` true _returnvalue)
            (bind _returnvalue_4 (`|CreateWidget` "/Game/UI/Timer.Timer_C"))
            (`UserWidget.AddToViewport` _returnvalue_4 0)
            (`KismetSystemLibrary.Delay` 120.0)
            (`WidgetLayoutLibrary.RemoveAllWidgets`)
            (bind _returnvalue_5 (`|CreateWidget` "/Game/UI/Inventory.Inventory_C"))
            (`UserWidget.AddToViewport` _returnvalue_5 0)
            (bind _returnvalue_6 (`|CreateWidget` "/Game/UI/Timer.Timer_C"))
            (`UserWidget.AddToViewport` _returnvalue_6 0)
            (set `PlayerController.bShowMouseCursor` false _returnvalue_2)
            (`WidgetBlueprintLibrary.SetInputMode_GameOnly` _returnvalue_2)
            (set `self.DoorTo3rdRoom` true)))))))

(fn `UserConstructionScript`)