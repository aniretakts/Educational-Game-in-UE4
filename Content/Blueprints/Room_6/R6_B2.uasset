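; Room 6 board actor that opens the R6_Q2 question widget when the player presses Enter inside its trigger.
; The first press shows the question and Timer with UI-only input, then a fixed 30-second Delay restores Inventory, Timer and game input.
; It then increments DoorTo7thRoom on an R6_B1 actor without checking any answer.
; Later presses only reveal a text and plane, hidden again on leaving the trigger.
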(event `self.3rdRoomBoardTrigger.OnComponentBeginOverlap`
  (params (OverlappedComponent :type "PrimitiveComponent Object Reference") (OtherActor :type "Actor Object Reference") (OtherComp :type "PrimitiveComponent Object Reference") (OtherBodyIndex :type Integer) (bFromSweep :type Boolean) (SweepResult :type "HitResult Structure (by ref)"))
  (`self.EnableInput` (`GameplayStatics.GetPlayerController` 0)))

(event `self.3rdRoomBoardTrigger.OnComponentEndOverlap`
  (params (OverlappedComponent :type "PrimitiveComponent Object Reference") (OtherActor :type "Actor Object Reference") (OtherComp :type "PrimitiveComponent Object Reference") (OtherBodyIndex :type Integer))
  (`self.DisableInput` (`GameplayStatics.GetPlayerController` 0))
  (`SceneComponent.SetHiddenInGame` (`self.TextRender1`) true false)
  (`SceneComponent.SetHiddenInGame` (`self.Plane`) true false))

(event `Key|Enter`
  (params (Key :type "Key Structure"))
  (bind _returnvalue (`GameplayStatics.GetPlayerController` 0))
  (bind _returnvalue_2 (`GameplayStatics.GetPlayerController` 0))
  (:`Pressed`
    (`/Engine/EditorBlueprintResources/StandardMacros.IncrementInt` (`self.counter`)
      (:`  `
        (if (>= (`self.counter`) 2)
          (`SceneComponent.SetHiddenInGame` (`self.TextRender1`) false false)
          (`SceneComponent.SetHiddenInGame` (`self.Plane`) false false)
          (else
            (set `self.R6Q2Triggered` true)
            (`WidgetLayoutLibrary.RemoveAllWidgets`)
            (bind _returnvalue_3 (`|CreateWidget` "/Game/Blueprints/Room_6/R6_Q2.R6_Q2_C"))
            (`UserWidget.AddToViewport` _returnvalue_3 0)
            (`WidgetBlueprintLibrary.SetInputMode_UIOnlyEx` _returnvalue null)
            (set `PlayerController.bShowMouseCursor` true _returnvalue)
            (bind _returnvalue_4 (`|CreateWidget` "/Game/UI/Timer.Timer_C"))
            (`UserWidget.AddToViewport` _returnvalue_4 0)
            (`KismetSystemLibrary.Delay` 30.0)
            (`WidgetLayoutLibrary.RemoveAllWidgets`)
            (bind _returnvalue_5 (`|CreateWidget` "/Game/UI/Inventory.Inventory_C"))
            (`UserWidget.AddToViewport` _returnvalue_5 0)
            (bind _returnvalue_6 (`|CreateWidget` "/Game/UI/Timer.Timer_C"))
            (`UserWidget.AddToViewport` _returnvalue_6 0)
            (set `PlayerController.bShowMouseCursor` false _returnvalue_2)
            (`WidgetBlueprintLibrary.SetInputMode_GameOnly` _returnvalue_2)
            (bind _outactors (`GameplayStatics.GetAllActorsOfClass` "/Game/Blueprints/Room_6/R6_B1.R6_B1_C"))
            (for _array_element _outactors
              _)
            (set `/Game/Blueprints/Room_6/R6_B1.DoorTo7thRoom` (+ (`/Game/Blueprints/Room_6/R6_B1.DoorTo7thRoom` _array_element) 1) _array_element)))))))

(fn `UserConstructionScript`)