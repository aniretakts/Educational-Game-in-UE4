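; Room 5 board actor that presents the room's third quiz question when the player presses Enter inside its trigger, which toggles input on overlap.
; Enter swaps the UI to the question and timer widgets with mouse control, then restores inventory, timer and game input after a fixed delay.
; It then increments the R5_B1 actor's sixth-room door counter, compares that actor's stored answers to the correct ones by index, and prints a percentage score.
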(event `self.3rdRoomBoardTrigger.OnComponentBeginOverlap`
  (params (OverlappedComponent :type "PrimitiveComponent Object Reference") (OtherActor :type "Actor Object Reference") (OtherComp :type "PrimitiveComponent Object Reference") (OtherBodyIndex :type Integer) (bFromSweep :type Boolean) (SweepResult :type "HitResult Structure (by ref)"))
  (`self.EnableInput` (`GameplayStatics.GetPlayerController` 0)))

(event `self.3rdRoomBoardTrigger.OnComponentEndOverlap`
  (params (OverlappedComponent :type "PrimitiveComponent Object Reference") (OtherActor :type "Actor Object Reference") (OtherComp :type "PrimitiveComponent Object Reference") (OtherBodyIndex :type Integer))
  (`self.DisableInput` (`GameplayStatics.GetPlayerController` 0)))

(event `Key|Enter`
  (params (Key :type "Key Structure"))
  (bind _returnvalue (`GameplayStatics.GetPlayerController` 0))
  (bind _returnvalue_2 (`GameplayStatics.GetPlayerController` 0))
  (:`Pressed`
    (set `self.R5Q3Triggered` true)
    (`WidgetLayoutLibrary.RemoveAllWidgets`)
    (bind _returnvalue_3 (`|CreateWidget` "/Game/Blueprints/Room_5/R5_Q3.R5_Q3_C"))
    (`UserWidget.AddToViewport` _returnvalue_3 0)
    (`WidgetBlueprintLibrary.SetInputMode_UIOnlyEx` _returnvalue null)
    (set `PlayerController.bShowMouseCursor` true _returnvalue)
    (bind _returnvalue_4 (`|CreateWidget` "/Game/UI/Timer.Timer_C"))
    (`UserWidget.AddToViewport` _returnvalue_4 0)
    (`KismetSystemLibrary.Delay` 30.0)
    (`WidgetLayoutLibrary.RemoveAllWidgets`)
    (bind _returnvalue_5 (`|CreateWidget` "/Game/UI/Inventory.Inventory_C"))
    (`UserWidget.AddToViewport` _returnvalue_5 0)
    (bind _returnvalue_6 (`|CreateWidget` "/Game/UI/Timer.Timer_C"))
    (`UserWidget.AddToViewport` _returnvalue_6 0)
    (set `PlayerController.bShowMouseCursor` false _returnvalue_2)
    (`WidgetBlueprintLibrary.SetInputMode_GameOnly` _returnvalue_2)
    (bind _outactors (`GameplayStatics.GetAllActorsOfClass` "/Game/Blueprints/Room_5/R5_B1.R5_B1_C"))
    (for _array_element _outactors
      _)
    (set `/Game/Blueprints/Room_5/R5_B1.DoorTo6thRoom` (+ (`/Game/Blueprints/Room_5/R5_B1.DoorTo6thRoom` _array_element) 1) _array_element)
    (for (_array_element_2 _array_index) (`/Game/Blueprints/Room_5/R5_B1.UsersAnswersR5` _array_element)
      (for (_array_element_3 _array_index_2) (`self.R5CorrectAnswers`)
        (if (== _array_index_2 _array_index)
          (if (`KismetStringLibrary.EqualEqual_StrStr` _array_element_3 _array_element_2)
            (bind _output_get (set `self.R5NumOfCorrectAnswers` (+ (`self.R5NumOfCorrectAnswers`) 1)))
            (bind _output_get_2 (set `self.R5Score` (/ (* _output_get 100) 3)))))))
    (`KismetSystemLibrary.PrintString` "Your score in percentage is:" true true (struct :`G` 0.66 :`B` 1.0 :`A` 1.0) 20.0)
    (`KismetSystemLibrary.PrintString` (`KismetStringLibrary.Conv_IntToString` _output_get_2) true true (struct :`G` 0.66 :`B` 1.0 :`A` 1.0) 20.0)))

(fn `UserConstructionScript`)