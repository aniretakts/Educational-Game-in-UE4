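; R2_Result is an actor Blueprint that scores the player's answers for Room 2 when a 2ndRoom_Board overlaps it.
; Nested loops compare the board's correct and user answer arrays at matching indices, incrementing CorAns for each match.
; It converts CorAns to a percentage of a hardcoded seven questions and prints both values as debug text.
; CorAns is never reset here, so repeated overlaps accumulate the count.
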(event `self.ReceiveBeginPlay`)

(event `self.ReceiveActorBeginOverlap`
  (params (OtherActor :type "Actor Object Reference"))
  (bind _as2nd_room_board (cast `/Game/Blueprints/Room_2/2ndRoom_Board` OtherActor))
  (for (_array_element _array_index) (`/Game/Blueprints/Room_2/2ndRoom_Board.R2CorrectAnswers` _as2nd_room_board)
    (for (_array_element_2 _array_index_2) (`/Game/Blueprints/Room_2/2ndRoom_Board.R2UsersAnswers` _as2nd_room_board)
      (if (== _array_index_2 _array_index)
        (if (`KismetStringLibrary.EqualEqual_StrStr` _array_element_2 _array_element)
          (set `self.corAns` (+ (`self.corAns`) 1))))))
  (set `self.result` (/ (* (`self.corAns`) 100) 7))
  (`KismetSystemLibrary.PrintString` (`KismetStringLibrary.Conv_IntToString` (`self.result`)) true true (struct :`G` 0.66 :`B` 1.0 :`A` 1.0) 20.0)
  (`KismetSystemLibrary.PrintString` (`KismetStringLibrary.Conv_IntToString` (`self.corAns`)) true true (struct :`R` 1.0 :`B` 0.938075 :`A` 1.0) 20.0))

(fn `UserConstructionScript`)