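; BP_6th_Door is a door that swings open on trigger overlap once the DoorTo6thRoom value on R5_B1 equals 3.
; Otherwise it shows a text hint, which hides again when the overlap ends.
; The DoorOpen timeline yaws the door and disables BlockVolume collision, then a 10-second Delay fired from its update leads into DoorClose, which rotates it back and restores collision.
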(event `self.OpenDoorTrigger.OnComponentBeginOverlap`
  (params (OverlappedComponent :type "PrimitiveComponent Object Reference") (OtherActor :type "Actor Object Reference") (OtherComp :type "PrimitiveComponent Object Reference") (OtherBodyIndex :type Integer) (bFromSweep :type Boolean) (SweepResult :type "HitResult Structure (by ref)"))
  (`self.EnableInput` (`GameplayStatics.GetPlayerController` 0))
  (bind _outactors (`GameplayStatics.GetAllActorsOfClass` "/Game/Blueprints/Room_5/R5_B1.R5_B1_C"))
  (for _array_element _outactors
    _)
  (if (== (`/Game/Blueprints/Room_5/R5_B1.DoorTo6thRoom` _array_element) 3)
    (bind (_direction _output) (`Timeline|DoorOpen`)
      (:`Update`
        (`SceneComponent.K2_SetRelativeRotation` (`self.SM_Door`) (`KismetMathLibrary.MakeRotator` 0.0 0.0 _output) false false)
        (`PrimitiveComponent.SetCollisionEnabled` (`self.BlockVolume`) "NoCollision")
        (`KismetSystemLibrary.Delay` 10.0)
        (bind (_direction_2 _newtrack_0) (`Timeline|DoorClose`)
          (:`Update`
            (`SceneComponent.K2_SetRelativeRotation` (`self.SM_Door`) (`KismetMathLibrary.MakeRotator` 0.0 0.0 _newtrack_0) false false)
            (`PrimitiveComponent.SetCollisionEnabled` (`self.BlockVolume`) "QueryAndPhysics")))))
    (else
      (`SceneComponent.SetHiddenInGame` (`self.Text`) false false))))

(event `self.OpenDoorTrigger.OnComponentEndOverlap`
  (params (OverlappedComponent :type "PrimitiveComponent Object Reference") (OtherActor :type "Actor Object Reference") (OtherComp :type "PrimitiveComponent Object Reference") (OtherBodyIndex :type Integer))
  (`self.DisableInput` (`GameplayStatics.GetPlayerController` 0))
  (`SceneComponent.SetHiddenInGame` (`self.Text`) true false))

(fn `UserConstructionScript`)